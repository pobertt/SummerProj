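; Base weapon actor for an FPS character that fires single or automatic shots and tracks magazine ammo.
; Automatic fire loops on a delay while the player is shooting; each shot plays sound, a normal or last-round montage and camera shake.
; Hitscan traces from the camera, then from the muzzle toward that trace's end point with optional debug drawing, without applying damage.
; Equip, Stow, Reload and StopFire are empty events.
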(event `self.ReceiveBeginPlay`
  (bind _asbp_fpscharacter (cast `/Game/Player/Character/BP_FPSCharacter` (`self.GetParentActor`)))
  (set `self.PlayerRef` _asbp_fpscharacter)
  (set `self.CurrentAmmo` (`self.MagSize`)))

(event `Equip`)

(event `Stow`)

(event `Reload`)

(event `Fire`
  (switch `/Game/Weapons/E_FireMode` (`self.FireMode`)
    (:`NewEnumerator0`
      (`self.StartFire`)
      (`self.StopFire`))
    (:`NewEnumerator1`
      (if (`/Game/Player/Character/BP_FPSCharacter.Shooting?` (`self.PlayerRef`)) :!label _label
        (`self.StartFire`)
        (`KismetSystemLibrary.Delay` (`self.FireDelay`))
        (goto _label)))))

(event `StopFire`)

(event `StartFire`
  (bind _returnvalue (`self.K2_GetActorLocation`))
  (bind _animmontages_firemontage (break `/Game/Player/Anims/FPSCharacter/Structures/S_WeaponMontages` (`self.AnimMontages`)))
  (bind (_animmontages_firemontage_2 _animmontages_firelastmontage) (break `/Game/Player/Anims/FPSCharacter/Structures/S_WeaponMontages` (`self.AnimMontages`)))
  (bind _returnvalue_2 (- (`self.CurrentAmmo`) 1))
  (bind _firstpersonmesh (`/Game/Player/Character/BP_FPSCharacter.FirstPersonMesh` (`self.PlayerRef`)))
  (if (> _returnvalue_2 0)
    (`GameplayStatics.PlaySoundAtLocation` (`self.FireSound`) _returnvalue (struct) 1.0 1.0 0.0 null null null null)
    (`|PlayMontage` _firstpersonmesh _animmontages_firemontage
      (:`then`
        (set `self.CurrentAmmo` (- (`self.CurrentAmmo`) 1) :!label _label_2)
        (`self.FireHitScan` true)
        (`GameplayStatics.PlayWorldCameraShake` "/Game/CameraShake/CS_Fire.CS_Fire_C" (`self.K2_GetActorLocation` (`self.PlayerRef`)) 0.0 70.0)))
    (elif (== _returnvalue_2 0)
      (`GameplayStatics.PlaySoundAtLocation` (`self.FireSound`) _returnvalue (struct) 1.0 1.0 0.0 null null null null)
      (`|PlayMontage` _firstpersonmesh _animmontages_firelastmontage
        (:`then`
          (goto _label_2)))
      (else
        (`GameplayStatics.PlaySoundAtLocation` (`self.EmpySound`) (`self.K2_GetActorLocation`) (struct) 1.0 1.0 0.0 null null null null)
        (`self.StopFire`)))))

(fn `FireHitScan`
  (params (DrawDebug :type Boolean))
  (bind _camera (`/Game/Player/Character/BP_FPSCharacter.Camera` (`self.PlayerRef`)))
  (bind _returnvalue (`SceneComponent.K2_GetComponentLocation` _camera))
  (bind _outhit (`KismetSystemLibrary.LineTraceSingle` _returnvalue (+ _returnvalue (* (`SceneComponent.GetForwardVector` _camera) (`self.Range`))) "TraceTypeQuery1" false (`|MakeArray` self (`self.PlayerRef`) :!type "Actor Object Reference")))
  (bind (_bblockinghit _binitialoverlap _time _distance _location _impactpoint _normal _impactnormal _physmat _hitactor _hitcomponent _hitbonename _bonename _hititem _elementindex _faceindex _tracestart _traceend) (`GameplayStatics.BreakHitResult` _outhit))
  (`KismetSystemLibrary.LineTraceSingle` :`Start` (`SceneComponent.GetSocketLocation` (`self.Weapon_Mesh`) "Muzzle") :`End` (`KismetMathLibrary.SelectVector` _location _traceend) :`TraceChannel` "TraceTypeQuery1" :`DrawDebugType` (select `bool` (`local.DrawDebug`) :`true` "ForDuration" :!type "EDrawDebugTrace Enum"))
  (return))

(fn `UserConstructionScript`
  (`SkeletalMeshComponent.SetSkeletalMeshAsset` (`self.Weapon_Mesh`) (`self.Mesh`)))